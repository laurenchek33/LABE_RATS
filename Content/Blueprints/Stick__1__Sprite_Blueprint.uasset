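; A collectible stick sprite actor that the seagull player picks up on touch.
; On BeginPlay it binds to the player BP_ParentSeagull's DarkSideSet event, swapping its sprite between stick and scrap as the dark side state changes.
; When a BP_ParentSeagull overlaps its sphere, it increments that seagull's StickCount and destroys itself.
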(event `self.ReceiveBeginPlay`
  (bind _asbp_parent_seagull (cast `/Game/SEAGULLS/Characters/BP_ParentSeagull` (`GameplayStatics.GetPlayerPawn` 0)))
  (add `/Game/SEAGULLS/Characters/BP_ParentSeagull.DarkSideSet` _asbp_parent_seagull (delegate `DarkSideSet`)))

(event `DarkSideSet`
  (params (`is Dark Side` :type Boolean))
  (`PaperSpriteComponent.SetSprite` (`self.RenderComponent`) (select `bool` `is Dark Side` :`false` "/Game/Environment/sticks/Stick__1__Sprite.Stick__1__Sprite" :`true` "/Game/Environment/sticks/Scrap1_Sprite.Scrap1_Sprite" :!type "PaperSprite Object Reference")))

(event `self.Sphere.OnComponentBeginOverlap`
  (params (OverlappedComponent :type "PrimitiveComponent Object Reference") (OtherActor :type "Actor Object Reference") (OtherComp :type "PrimitiveComponent Object Reference") (OtherBodyIndex :type Integer) (bFromSweep :type Boolean) (SweepResult :type "HitResult Structure (by ref)"))
  (bind _asbp_parent_seagull (cast `/Game/SEAGULLS/Characters/BP_ParentSeagull` OtherActor))
  (`/Engine/EditorBlueprintResources/StandardMacros.IncrementInt` (`/Game/SEAGULLS/Characters/BP_ParentSeagull.StickCount` _asbp_parent_seagull)
    (:`  `
      (`self.K2_DestroyActor`))))

(fn `UserConstructionScript`)