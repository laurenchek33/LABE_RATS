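; Player character Blueprint for Princess Seia, a sprite-based character that walks sideways along the world X axis.
; On BeginPlay it adds the IM_Princess Enhanced Input mapping context to the first player controller, and IA_Walking feeds its value into movement input.
; Every tick it checks the X velocity and rotates the sprite to face the travel direction, keeping the last facing when stopped.
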(event `self.ReceiveBeginPlay`
  (bind _asplayer_controller (cast `PlayerController` (`GameplayStatics.GetPlayerController` 0)))
  (bind _returnvalue (pcsubsystem `EnhancedInputLocalPlayerSubsystem` _asplayer_controller))
  (`/Engine/EditorBlueprintResources/StandardMacros.IsValid` _returnvalue
    (:`Is Valid`
      (`EnhancedInputSubsystemInterface.AddMappingContext` _returnvalue "/Game/Character_Pics/Princess_Seia/Blueprints/IM_Princess.IM_Princess" 0 (struct)))))

(event `self.ReceiveTick`
  (params (DeltaSeconds :type "Float (single-precision)"))
  (`self.Update Player Rotation`))

(event `Update Player Rotation`
  (bind _sprite (`self.Sprite`))
  (bind _velocity_x (`KismetMathLibrary.BreakVector` (`MovementComponent.Velocity` (`self.CharacterMovement`))))
  (`/Engine/EditorBlueprintResources/StandardMacros.CompareFloat` _velocity_x
    (:`>`
      (`SceneComponent.K2_SetRelativeRotation` _sprite (struct :`Yaw` 180.0) false false))
    (:`<`
      (`SceneComponent.K2_SetRelativeRotation` :`self` _sprite))))

(event `EnhancedInput|/Game/Character_Pics/Princess_Seia/Blueprints/IA_Walking`
  (params (ActionValue :type "Float (double-precision)") (ElapsedSeconds :type "Float (double-precision)") (TriggeredSeconds :type "Float (double-precision)") (InputAction :type "InputAction Object Reference" :default "/Game/Character_Pics/Princess_Seia/Blueprints/IA_Walking.IA_Walking"))
  (:`Triggered`
    (`self.AddMovementInput` (1.0 0.0 0.0) ActionValue)))

(fn `UserConstructionScript`)